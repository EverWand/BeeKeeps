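; Bee actor that seeks out the third-person player character and homes in on it by physics impulses.
; Until it has a valid target, Tick runs a sphere overlap around the bee and keeps the first character found.
; It then turns Body toward the target and applies a forward velocity-change impulse every frame.
; A self-repeating Charge event adds stronger or weaker bursts (ChargeStrength) at random delays, with or without a target.
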(event `Charge`
  (`KismetSystemLibrary.Delay` (`KismetArrayLibrary.Array_Random` (`self.Charge Delays`)))
  (`self.FlyFoward` (`self.ChargeStrength`))
  (`self.Charge`))

(event `self.ReceiveBeginPlay`
  (`self.Charge`))

(event `self.ReceiveTick`
  (params (DeltaSeconds :type "Float (single-precision)"))
  (bind _target (`self.Target`))
  (`/Engine/EditorBlueprintResources/StandardMacros.IsValid` _target
    (:`Is Valid`
      (`SceneComponent.K2_SetWorldRotation` (`self.Body`) (`KismetMathLibrary.FindLookAtRotation` (`SceneComponent.K2_GetComponentLocation` (`self.Body`)) (`self.K2_GetActorLocation` _target)) false false)
      (`self.FlyFoward` (`self.FlyStrength`)))
    (:`Is Not Valid`
      (bind (_found _didfind_) (`self.Look For Player`))
      (if _didfind_
        (set `self.Target` _found)))))

(fn `FlyFoward`
  (params (FlyStrength :type "Float (double-precision)"))
  (bind _body (`self.Body`))
  (`PrimitiveComponent.AddImpulse` _body (* FlyStrength (`SceneComponent.GetForwardVector` _body)) "None" true))

(fn `Look For Player`
  (returns (Found :type "Actor Object Reference") (`DidFind?` :type Boolean))
  (locals (NewLocalVar :type "Array of EObjectTypeQuery Enum"))
  (bind (_outactors _returnvalue) (`KismetSystemLibrary.SphereOverlapActors` (`self.K2_GetActorLocation`) 500.0 (`local.NewLocalVar`) "/Game/ThirdPerson/Blueprints/BP_ThirdPersonCharacter.BP_ThirdPersonCharacter_C"))
  (return (`|GetArrayItem` _outactors) _returnvalue))

(fn `UserConstructionScript`)